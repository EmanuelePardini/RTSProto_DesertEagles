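; Showcase Blueprint for the East D-30 122mm artillery piece, mapping generic checkbox, button and slider events to damage display, firing and part posing.
; Sliders drive speed, legs, suspension, gun elevation, holder angle, standing gear and turning wheels.
; Interlock flags chain the motions: near-zero leg angle unlocks suspension and standing gear, high suspension angle unlocks legs, and near-zero suspension enables speed, which is otherwise zeroed.
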(event `/Game/Assets/VigilanteContent/Shared/Blueprints/Showcase/Interfaces/BP_ShowcaseControlsInterface.SetCheckboxVariable0`
  (params (NewState :type Boolean))
  ;[1 1 1] Damaged model visibility
  (`self.Show Damaged` NewState)
  (set `self.DamagedFlag` NewState))

(event `/Game/Assets/VigilanteContent/Shared/Blueprints/Showcase/Interfaces/BP_ShowcaseControlsInterface.SetSliderVariable0`
  (params (NewValue :type "Float (double-precision)"))
  ;[1 1 1] Set Speed
  (if (`self.FlagToActivateSpeed`)
    (`self.Set Speed` NewValue)
    (else
      (`self.Set Speed` 0.0))))

(event `/Game/Assets/VigilanteContent/Shared/Blueprints/Showcase/Interfaces/BP_ShowcaseControlsInterface.SetButtonsVariable0`
  (params (NewIndex :type Integer))
  ;[1 1 1] Firing activation
  (`self.SetFiringActive`))

(event `/Game/Assets/VigilanteContent/Shared/Blueprints/Showcase/Interfaces/BP_ShowcaseControlsInterface.SetSliderVariable1`
  (params (NewValue :type "Float (double-precision)"))
  ;[1 1 1] Set legs angle
  (if (`self.CanLegsBeClosed?`)
    (`self.Set Legs Angle` NewValue)
    (if (and (>= NewValue -5.0) (<= NewValue 5.0))
      (set `self.FlagToDropWheels` true)
      (else
        (set `self.FlagToDropWheels` false)))))

(event `/Game/Assets/VigilanteContent/Shared/Blueprints/Showcase/Interfaces/BP_ShowcaseControlsInterface.SetSliderVariable2`
  (params (NewValue :type "Float (double-precision)"))
  ;[1 1 1] Set Suspension angle
  (if (`self.FlagToDropWheels`)
    (`self.SetSuspensionAngle` NewValue)
    (set `self.CanLegsBeClosed?` (>= NewValue 55.0))
    (if (<= NewValue 2.0)
      (set `self.FlagToActivateSpeed` true)
      (else
        (set `self.FlagToActivateSpeed` false)
        (`self.Set Speed` 0.0)))))

(event `/Game/Assets/VigilanteContent/Shared/Blueprints/Showcase/Interfaces/BP_ShowcaseControlsInterface.SetSliderVariable3`
  (params (NewValue :type "Float (double-precision)"))
  ;[1 1 1] Set variables: Gun elevation and Gun Holder Angle, wheel rotation, and gear displacement
  (`self.SetGunElevation` NewValue))

(event `/Game/Assets/VigilanteContent/Shared/Blueprints/Showcase/Interfaces/BP_ShowcaseControlsInterface.SetSliderVariable4`
  (params (NewValue :type "Float (double-precision)"))
  ;[1 1 1] Set variables: Gun elevation and Gun Holder Angle, wheel rotation, and gear displacement
  (`self.SetGunHolderAngle` NewValue))

(event `/Game/Assets/VigilanteContent/Shared/Blueprints/Showcase/Interfaces/BP_ShowcaseControlsInterface.SetSliderVariable5`
  (params (NewValue :type "Float (double-precision)"))
  ;[1 1 1] Set variables: Gun elevation and Gun Holder Angle, wheel rotation, and gear displacement
  (if (`self.FlagToDropWheels`)
    (`self.Standing Gear Displacement` NewValue)))

(event `/Game/Assets/VigilanteContent/Shared/Blueprints/Showcase/Interfaces/BP_ShowcaseControlsInterface.SetTwinSliderVariable0`
  (params (`bFirstSlider?` :type Boolean) (NewFirstValue :type "Float (double-precision)") (NewSecondValue :type "Float (double-precision)"))
  ;[1 1 1] Set variables: Gun elevation and Gun Holder Angle, wheel rotation, and gear displacement
  (if `bFirstSlider?`
    (`self.Set Turning Wheel Rotation Front` NewFirstValue)
    (else
      (`self.Set Truning Wheel Rotation Side` NewSecondValue))))

(fn `UserConstructionScript`
  (`parent.UserConstructionScript`))