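; BP_Nuclear is a short-lived nuclear strike actor that wipes out units around the spot where it is placed.
; Two seconds after BeginPlay, it gathers every UnitCharacter and destroys those within AttenuationRadius, measured by horizontal distance so height is ignored.
; Units are destroyed outright with no damage step or team check, then the actor destroys itself.
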(event `self.ReceiveBeginPlay`
  (`KismetSystemLibrary.Delay` 2.0)
  (bind _outactors (`GameplayStatics.GetAllActorsOfClass` "/Script/Consegna02_Pardini.UnitCharacter"))
  (for _array_element _outactors
    (if (<= (`KismetMathLibrary.Distance2D` (`KismetMathLibrary.Conv_VectorToVector2D` (`self.K2_GetActorLocation` _array_element)) (`KismetMathLibrary.Conv_VectorToVector2D` (`self.K2_GetActorLocation`))) (`self.AttenuationRadius`))
      (`self.K2_DestroyActor` _array_element)))
  (`self.K2_DestroyActor`))

(fn `UserConstructionScript`)